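; Enemy character Blueprint that passes its EnemyType to the AI_Controller on BeginPlay and drives AI through Blackboard keys.
; Damage lowers Health and updates a widget health bar; a hit arriving at zero Health or below flags death and destroys the bar.
; PawnSensing sets SeePlayer and AlertState on spotting the player.
; Tick yaws the bar toward the player while both are alive.
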(event `self.ReceiveBeginPlay`
  (bind _asai_controller (cast `/Game/Enemy/BehaviorTree/AI_Controller` (`self.GetController`)))
  (`/Game/Enemy/BehaviorTree/AI_Controller.SetEnemyType` _asai_controller (`self.EnemyType`)))

(event `self.ReceiveAnyDamage`
  (params (Damage :type "Float (single-precision)") (DamageType :type "DamageType Object Reference") (InstigatedBy :type "Controller Object Reference") (DamageCauser :type "Actor Object Reference"))
  (bind _returnvalue (> (`self.Health`) 0.0))
  ; Actualizacion de vida al recibir daño
  (if _returnvalue
    (set `self.Health` (- (`self.Health`) Damage))
    (if _returnvalue
      (bind _ashealth_bar_enemy (cast `/Game/UI/HealthBarEnemy` (`WidgetComponent.GetUserWidgetObject` (`self.HealthBar`))))
      (`ProgressBar.SetPercent` (`/Game/UI/HealthBarEnemy.ProgressBar_0` _ashealth_bar_enemy) (/ (`self.Health`) 100.0)))
    (else
      ; Muerte del enemigo
      (`BlackboardComponent.SetValueAsBool` (`AIBlueprintHelperLibrary.GetBlackboard` self) "IsDeath?" true)
      (`ActorComponent.K2_DestroyComponent` (`self.HealthBar`)))))

(event `self.ReceiveTick`
  (params (DeltaSeconds :type "Float (single-precision)"))
  (bind (_returnvalue_roll _returnvalue_pitch _returnvalue_yaw) (`KismetMathLibrary.BreakRotator` (`KismetMathLibrary.FindLookAtRotation` (`SceneComponent.K2_GetComponentLocation` (`self.HealthBar`)) (`self.K2_GetActorLocation` (`GameplayStatics.GetPlayerCharacter` 0)))))
  ; Verificar que el enemigo y el player esten vivos
  (if (> (`self.Health`) 0.0)
    (bind _asbp_third_person_character (cast `/Game/ThirdPerson/Blueprints/BP_ThirdPersonCharacter` (`GameplayStatics.GetPlayerCharacter` 0)))
    (if (> (`/Game/ThirdPerson/Blueprints/BP_ThirdPersonCharacter.Health` _asbp_third_person_character) 0.0)
      ; Asignar la rotacion de la barra de vida
      (`SceneComponent.K2_SetWorldRotation` (`self.HealthBar`) (`KismetMathLibrary.MakeRotator` 0.0 0.0 _returnvalue_yaw) false false))))

(event `self.PawnSensing.OnSeePawn`
  (params (Pawn :type "Pawn Object Reference"))
  (bind _returnvalue (`AIBlueprintHelperLibrary.GetBlackboard` (`AIBlueprintHelperLibrary.GetAIController` self)))
  ; Activar comportamiento de perseguir al jugador
  (cast `/Game/ThirdPerson/Blueprints/BP_ThirdPersonCharacter` Pawn)
  (`BlackboardComponent.SetValueAsBool` _returnvalue "SeePlayer?" true)
  (`BlackboardComponent.SetValueAsBool` _returnvalue "AlertState" true))

(fn `UserConstructionScript`)